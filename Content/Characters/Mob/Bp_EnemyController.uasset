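; Bp_EnemyController is an AI controller for Bp_Mob enemies that drives them with the BT_Flying behavior tree.
; On BeginPlay it starts the tree, caches the controlled mob and writes its starting location to the HomeLocation blackboard key.
; A SetTarget event lets other code write an object to the Target blackboard key.
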(event `self.ReceiveBeginPlay`
  (`self.RunBehaviorTree` "/Game/Characters/Mob/BT_Flying.BT_Flying")
  (bind _asbp_mob (cast `/Game/Characters/Mob/Bp_Mob` (`self.K2_GetPawn`)))
  (set `self.Mob` _asbp_mob)
  (`BlackboardComponent.SetValueAsVector` (`self.Blackboard`) "HomeLocation" (`self.K2_GetActorLocation` (`self.Mob`))))

(event `SetTarget`
  (params (Target :type "/Game/Characters/Human/Ch_Base Object Reference"))
  (`BlackboardComponent.SetValueAsObject` (`self.Blackboard`) "Target" Target))

(fn `UserConstructionScript`)