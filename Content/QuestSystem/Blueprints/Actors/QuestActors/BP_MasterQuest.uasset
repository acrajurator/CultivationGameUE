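; Master quest actor that tracks a quest's active and completed sub-goals from its QuestInfo data.
; Active goals are held as indices into the sub-goal list, seeded from starting indices or advanced sequentially by GoToNextSubGoal.
; CompleteSubGoal records success, activates the goal's following indices to allow branching, and directly swaps the quest widget's entries.
; Completing the selected goal of the manager's current quest reselects the first sub-goal widget.
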(fn `CompleteSubGoal`
  (params (SubGoalIndex :type Integer))
  (returns (Success :type Boolean))
  (locals (localGoalIndex :type Integer) (localCompletedGoal :type "/Game/QuestSystem/Blueprints/Structures/S_GoalInfo Structure") (localWidgetIndex :type Integer :default 0))
  (bind _questwidget (`self.QuestWidget`))
  (bind _questwidget_2 (`self.QuestWidget`))
  (bind _currentgoalindices (`self.CurrentGoalIndices`))
  (bind _subgoalwidgets (`/Game/QuestSystem/Widgets/QuestWidget.SubGoalWidgets` (`self.QuestWidget`)))
  (set `local.localGoalIndex` SubGoalIndex)
  (if (`KismetArrayLibrary.Array_Contains` (`self.CurrentGoalIndices`) (`local.localGoalIndex`))
    (bind _output_get (set `local.localCompletedGoal` (`|GetArrayItem` (`.SubGoals_28_B724667F4AA28F6C7281728692C07079` (break `/Game/QuestSystem/Blueprints/Structures/S_QuestInfo` (`self.QuestInfo`))) (`local.localGoalIndex`))))
    (`KismetArrayLibrary.Array_Add` (`self.CompletedSubGoals`) (make `/Game/QuestSystem/Blueprints/Structures/S_CompletedGoal` (`local.localGoalIndex`) _output_get true))
    (`KismetArrayLibrary.Array_RemoveItem` (`self.CurrentGoals`) (`local.localCompletedGoal`))
    (set `local.localWidgetIndex` (`KismetArrayLibrary.Array_Find` _currentgoalindices (`local.localGoalIndex`)))
    (`KismetArrayLibrary.Array_RemoveItem` _currentgoalindices (`local.localGoalIndex`))
    (`Widget.RemoveFromParent` (`|GetArrayItem` _subgoalwidgets (`local.localWidgetIndex`)))
    (`KismetArrayLibrary.Array_Remove` _subgoalwidgets (`local.localWidgetIndex`))
    (for _array_element (`.FollowingSubGoalIndices_26_2B7BE649487E86F2FA3ADE90C3FDA143` (break `/Game/QuestSystem/Blueprints/Structures/S_GoalInfo` (`local.localCompletedGoal`)))
      (`KismetArrayLibrary.Array_Add` (`self.CurrentGoalIndices`) _array_element)
      (bind _output (`|GetArrayItem` (`.SubGoals_28_B724667F4AA28F6C7281728692C07079` (break `/Game/QuestSystem/Blueprints/Structures/S_QuestInfo` (`self.QuestInfo`))) _array_element))
      (`KismetArrayLibrary.Array_Add` (`self.CurrentGoals`) _output)
      (bind _returnvalue (`|CreateWidget` "/Game/QuestSystem/Widgets/SubGoalWidget.SubGoalWidget_C" null _output self _questwidget))
      (`KismetArrayLibrary.Array_Add` (`/Game/QuestSystem/Widgets/QuestWidget.SubGoalWidgets` _questwidget) _returnvalue)
      (`PanelWidget.AddChild` (`/Game/QuestSystem/Widgets/QuestWidget.SubGoalBox` _questwidget) _returnvalue))
    (if (and (== (`local.localGoalIndex`) (`self.SelectedSubGoalIndex`)) (== (`/Game/QuestSystem/Blueprints/Actors/BP_QuestManager.CurrentQuest` (`self.QuestManager`)) self))
      (`/Game/QuestSystem/Widgets/QuestWidget.SelectSubGoal` _questwidget_2 (`|GetArrayItem` (`/Game/QuestSystem/Widgets/QuestWidget.SubGoalWidgets` _questwidget_2)))
      (return true)
      (else
        (return true)))
    (else
      (return false))))

(fn `GoToNextSubGoal`
  (returns (Success :type Boolean))
  (locals (NextIndex :type Integer :default 0))
  (bind _currentgoalindices (`self.CurrentGoalIndices`))
  (bind _returnvalue (+ (`.MaxValue` (`KismetMathLibrary.MaxOfIntArray` (`self.CurrentGoalIndices`))) 1))
  (if (<= _returnvalue (`KismetArrayLibrary.Array_LastIndex` (`.SubGoals_28_B724667F4AA28F6C7281728692C07079` (break `/Game/QuestSystem/Blueprints/Structures/S_QuestInfo` (`self.QuestInfo`)))))
    (set `local.NextIndex` _returnvalue)
    (`KismetArrayLibrary.Array_Clear` _currentgoalindices)
    (`KismetArrayLibrary.Array_Add` _currentgoalindices (`local.NextIndex`))
    (`self.UpdateSubGoals`)
    (return true)
    (else
      (return false))))

(fn `SetupStartingGoals`
  (`KismetArrayLibrary.Array_Clear` (`self.CurrentGoalIndices`))
  (set `self.CurrentGoalIndices` (`self.StartingSubGoalIndices`))
  (`self.UpdateSubGoals`)
  (set `self.CurrentDescription` (`.Description_8_090C71B944923055CD1F3AB8A65FAD83` (break `/Game/QuestSystem/Blueprints/Structures/S_QuestInfo` (`self.QuestInfo`))))
  (return))

(fn `UpdateSubGoals`
  (`KismetArrayLibrary.Array_Clear` (`self.CurrentGoals`))
  (for _array_element (`self.CurrentGoalIndices`)
    (`KismetArrayLibrary.Array_Add` (`self.CurrentGoals`) (`|GetArrayItem` (`.SubGoals_28_B724667F4AA28F6C7281728692C07079` (break `/Game/QuestSystem/Blueprints/Structures/S_QuestInfo` (`self.QuestInfo`))) _array_element)))
  (return))

(fn `UserConstructionScript`)