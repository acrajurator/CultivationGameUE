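; Quest manager actor that adds quests to the game and tracks which one is currently selected.
; AddNewQuest rejects invalid or already-added classes, otherwise spawns a quest actor, sets up its goals, creates its list widget and reveals the main widget if slid out.
; A new quest becomes selected when flagged to start or when it is the only one.
; SelectNewQuest switches the highlighted quest and sub-goal in the UI.
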(event `OnSwitchSubQuest`)

(fn `AddNewQuest`
  (params (QuestClass :type "/Game/QuestSystem/Blueprints/Actors/QuestActors/BP_MasterQuest Class Reference") (DirectlyStart :type Boolean))
  (returns (Success :type Boolean))
  (locals (localClass :type "/Game/QuestSystem/Blueprints/Actors/QuestActors/BP_MasterQuest Class Reference") (localStart :type Boolean) (localQuestActor :type "/Game/QuestSystem/Blueprints/Actors/QuestActors/BP_MasterQuest Object Reference"))
  (bind _mainwidget (`self.MainWidget`))
  (bind _localquestactor (`local.localQuestActor`))
  (bind _localquestactor_2 (`local.localQuestActor`))
  (set `local.localClass` QuestClass)
  (set `local.localStart` DirectlyStart)
  (if (and (`KismetSystemLibrary.IsValidClass` QuestClass) (not (`KismetArrayLibrary.Array_Contains` (`self.AllQuestClasses`) QuestClass)))
    (`KismetArrayLibrary.Array_Add` (`self.AllQuestClasses`) (`local.localClass`))
    (bind _returnvalue (`|SpawnActorFromClass` (`local.localClass`) (`KismetMathLibrary.MakeTransform` (0.0 0.0 0.0)) "AlwaysSpawn" "OverrideRootScale" null self null))
    (bind _output_get (set `local.localQuestActor` _returnvalue))
    (`KismetArrayLibrary.Array_Add` (`self.CurrentQuestActors`) _output_get)
    (`/Game/QuestSystem/Blueprints/Actors/QuestActors/BP_MasterQuest.SetupStartingGoals` _localquestactor)
    (bind _widget (`/Game/QuestSystem/Widgets/MainWidget.AddQuestToList` (`self.MainWidget`) _localquestactor))
    (bind _output_get_2 (set `/Game/QuestSystem/Blueprints/Actors/QuestActors/BP_MasterQuest.QuestWidget` _widget _localquestactor))
    (`/Game/QuestSystem/Widgets/QuestWidget.UpdateQuest` _output_get_2)
    (if (or (`local.localStart`) (<= (`KismetArrayLibrary.Array_Length` (`self.CurrentQuestActors`)) 1))
      (`self.SelectNewQuest` _localquestactor_2 (`|GetArrayItem` (`/Game/QuestSystem/Widgets/QuestWidget.SubGoalWidgets` (`/Game/QuestSystem/Blueprints/Actors/QuestActors/BP_MasterQuest.QuestWidget` _localquestactor_2)))))
    (if (`/Game/QuestSystem/Widgets/MainWidget.SlideOut?` (`self.MainWidget`))
      (`UserWidget.PlayAnimation` _mainwidget (`/Game/QuestSystem/Widgets/MainWidget.SlideOut` _mainwidget) 0.0 1 "Reverse" 1.0 false)
      (set `/Game/QuestSystem/Widgets/MainWidget.SlideOut?` false _mainwidget)
      (return true)
      (else
        (return true)))
    (else
      (return false))))

(fn `SelectNewQuest`
  (params (Quest :type "/Game/QuestSystem/Blueprints/Actors/QuestActors/BP_MasterQuest Object Reference") (SubGoal :type "/Game/QuestSystem/Widgets/SubGoalWidget Object Reference"))
  (bind _currentquest (`self.CurrentQuest`))
  (bind _questwidget (`/Game/QuestSystem/Blueprints/Actors/QuestActors/BP_MasterQuest.QuestWidget` _currentquest))
  (`/Engine/EditorBlueprintResources/StandardMacros.IsValid` _currentquest
    (:`Is Valid`
      (`Widget.SetIsEnabled` (`/Game/QuestSystem/Widgets/QuestWidget.QuestName` _questwidget) false)
      (`/Game/QuestSystem/Widgets/QuestWidget.SelectSubGoal` _questwidget null))
    (:`Is Not Valid`
      _))
  (bind _output_get (set `self.CurrentQuest` Quest))
  (`/Game/QuestSystem/Widgets/QuestWidget.OnQuestSelected` (`/Game/QuestSystem/Blueprints/Actors/QuestActors/BP_MasterQuest.QuestWidget` _output_get) SubGoal)
  (return))

(fn `UserConstructionScript`)