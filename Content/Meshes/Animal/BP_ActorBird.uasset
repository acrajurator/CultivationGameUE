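; BP_ActorBird is a bird actor that flies along the spline of a referenced Track actor.
; On BeginPlay, if ActiveBird is set, MoveBird scales the BirdLoop timeline's play rate by Duration and starts it at CartStartOffset.
; Each update maps the timeline's Alpha to a distance along the spline, then applies that world location with the spline's roll and yaw, leaving pitch at zero.
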(event `self.ReceiveBeginPlay`
  (if (`self.activeBird`)
    (`self.MoveBird`)))

(event `MoveBird`
  (bind _usefulspline (`/Game/Meshes/Animal/BP_Track.UsefulSpline` (`self.track`)))
  (bind _returnvalue (`KismetMathLibrary.Lerp` 0.0 (`SplineComponent.GetSplineLength` _usefulspline) (`self.alpha`)))
  (bind (_returnvalue_roll _returnvalue_pitch _returnvalue_yaw) (`KismetMathLibrary.BreakRotator` (`SplineComponent.GetRotationAtDistanceAlongSpline` _usefulspline _returnvalue "World")))
  (`TimelineComponent.SetPlayRate` (`self.BirdLoop`) (/ 1.0 (`self.duration`)))
  (`TimelineComponent.SetNewTime` (`self.BirdLoop`) (`self.cartStartOffset`))
  (bind (_direction _alpha) (`Timeline|BirdLoop`)
    (:`Update`
      (set `self.alpha` _alpha)
      (`self.K2_SetActorLocationAndRotation` (`SplineComponent.GetLocationAtDistanceAlongSpline` _usefulspline _returnvalue "World") (`KismetMathLibrary.MakeRotator` _returnvalue_roll 0.0 _returnvalue_yaw)))))

(fn `UserConstructionScript`)