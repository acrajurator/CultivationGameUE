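; Sword actor that travels along the spline of a referenced Track, following its position, yaw and roll.
; Shortly after BeginPlay it calls MoveSword regardless of ActiveSword, as both branch paths continue to the same call.
; MoveSword scales the TimeSwordLoop timeline rate by Duration and starts it at CartStartOffset.
; Each update maps the timeline's Alpha to a distance along the spline, leaving pitch unread.
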(event `self.ReceiveBeginPlay`
  (`KismetSystemLibrary.Delay` 0.2)
  (if (`self.activeSword`)
    _
    (else
      _))
  (`self.MoveSword`))

(event `MoveSword`
  (bind _timeswordloop (`self.TimeSwordLoop`))
  (bind _usefulspline (`/Game/Meshes/Animal/BP_Track.UsefulSpline` (`self.track`)))
  (bind _returnvalue (`KismetMathLibrary.Lerp` 0.0 (`SplineComponent.GetSplineLength` _usefulspline) (`self.alpha`)))
  (bind (_returnvalue_roll _returnvalue_pitch _returnvalue_yaw) (`KismetMathLibrary.BreakRotator` (`SplineComponent.GetRotationAtDistanceAlongSpline` _usefulspline _returnvalue "World")))
  (`TimelineComponent.SetPlayRate` _timeswordloop (/ 1.0 (`self.duration`)))
  (`TimelineComponent.SetNewTime` _timeswordloop (`self.cartStartOffset`))
  (bind (_direction _alpha) (`Timeline|TimeSwordLoop`)
    (:`Update`
      (set `self.alpha` _alpha)
      (`self.K2_SetActorLocationAndRotation` (`SplineComponent.GetLocationAtDistanceAlongSpline` _usefulspline _returnvalue "World") (`KismetMathLibrary.MakeRotator` _returnvalue_roll 0.0 _returnvalue_yaw)))))

(fn `UserConstructionScript`)